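; BP_WeaponPickup is a pickup that swaps the player's current weapon for a rifle when Equip is pressed in range.
; Collision overlap events cache the overlapping BP_JoyCharacter and toggle a CanPick flag.
; On Equip, it destroys the weapon through that character's WeaponComponent, spawns the hardcoded BP_RifleWeapon, then calls PickupWasTaken, which is not defined in this Blueprint.
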(event OnComponentBeginOverlap(Collision)
  (params (OverlappedComponent :type Primitive%20Component%20Object%20Reference) (OtherActor :type Actor%20Object%20Reference) (OtherComp :type Primitive%20Component%20Object%20Reference) (OtherBodyIndex :type Integer) (bFromSweep :type Boolean) (SweepResult :type Hit%20Result%20Structure%20%28by%20ref%29))
  (bind _asbp_joy_character (Utilities|Casting|CastToBP_JoyCharacter OtherActor))
  (Variables|Default|SetBPJoyCharacter _asbp_joy_character)
  (Variables|Default|SetCanPick true))

(event OnComponentEndOverlap(Collision)
  (params (OverlappedComponent :type Primitive%20Component%20Object%20Reference) (OtherActor :type Actor%20Object%20Reference) (OtherComp :type Primitive%20Component%20Object%20Reference) (OtherBodyIndex :type Integer))
  (Utilities|Casting|CastToBP_JoyCharacter OtherActor)
  (Variables|Default|SetCanPick false))

(event Input|ActionEvents|InputActionEquip
  (params (Key :type Key%20Structure :default "None"))
  (:Pressed
    (bind _bpjoycharacter (Variables|Default|GetBPJoyCharacter)
      (:then
        (if (Variables|Default|GetCanPick)
          (Class|WeaponComponent|DestoryWeapon (Variables|/Script/JoyTest.JoyCharacter|GetWeaponComponent _bpjoycharacter))
          (Class|WeaponComponent|SpawnWeapon (Variables|/Script/JoyTest.JoyCharacter|GetWeaponComponent _bpjoycharacter) "/Game/Weapons/BP_RifleWeapon.BP_RifleWeapon_C")
          (Class|BasePickupActor|PickupWasTaken)))
      (:else))))

(fn ConstructionScript)